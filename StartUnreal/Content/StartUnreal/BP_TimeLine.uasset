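; Blueprint actor that slides its Sphere back and forth along relative X using a Timeline.
; EventStart plays or reverses the Timeline based on IsMoveRight, and each update scales the curve value into the sphere's position.
; On finish it flips IsMoveRight and loops until EventStop halts it.
; DoPlay and DoStop extend the parent versions with inverted mapping: DoPlay calls EventStop and DoStop calls EventStart.
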(event `EventStart`
  (if (`self.IsMoveRight`) :!label _label
    (bind (_direction _value) (`Timeline|Timeline` :!label _label_2)
      (:`Update`
        (`SceneComponent.K2_SetRelativeLocation` (`self.Sphere`) (`KismetMathLibrary.MakeVector` (* _value 100.0)) false false))
      (:`Finished`
        (set `self.IsMoveRight` (not (`self.IsMoveRight`)))
        (goto _label)))
    (else
      (goto _label_2 :!via `Reverse`))))

(event `self.ReceiveBeginPlay`)

(event `EventStop`
  (goto _label_2 :!via `Stop`))

(fn `DoPlay`
  (`parent.DoPlay`)
  (`self.EventStop`))

(fn `DoStop`
  (`parent.DoStop`)
  (`self.EventStart`))

(fn `UserConstructionScript`)