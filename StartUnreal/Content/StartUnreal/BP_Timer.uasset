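; BP_Timer is a timer actor that shows elapsed time as MM:SS on a TextRender component.
; While IsPlay is set, Tick accumulates delta time at ten times real speed, deliberately sped up, and splits it into minutes and seconds.
; FloatToStr00 floors each value and zero-pads it to two digits.
; DoPlay and DoStop call their parent versions, then switch IsPlay on or off.
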(event `self.ReceiveTick`
  (params (DeltaSeconds :type "Float (single-precision)"))
  (if (`self.isPlay`)
    ;[1 1 1] 숫자 흐름이 빨리가게끔 일부로 곱해줌
    (bind _output_get (set `self.TotalDeltaSecond` (+ (* DeltaSeconds 10.0) (`self.TotalDeltaSecond`))))
    ;[1 1 1] 나누기 : 분 / 나머지 : 초
    (bind _str00 (`self.FloatToStr00` (/ _output_get 60.0)))
    (bind _str00_2 (`self.FloatToStr00` (mod _output_get 60.0)))
    ;[1 1 1] 분과 초를 나눠서 출력부분
    (`TextRenderComponent.K2_SetText` (`self.TextRender`) (`KismetTextLibrary.Conv_StringToText` (`KismetStringLibrary.Concat_StrStr` _str00 ":" _str00_2)))))

(fn `DoPlay`
  (`parent.DoPlay`)
  (set `self.isPlay` true))

(fn `DoStop`
  (`parent.DoStop`)
  (set `self.isPlay` false))

(fn `FloatToStr00`
  (params (Float :type "Float (double-precision)"))
  (returns (Str00 :type String))
  (bind _returnvalue (`KismetMathLibrary.FFloor` Float))
  (if (< _returnvalue 10)
    (return (`KismetStringLibrary.Concat_StrStr` "0" (`KismetStringLibrary.Conv_IntToString` _returnvalue)))
    (else
      (return (`KismetStringLibrary.Conv_IntToString` _returnvalue)))))

(fn `UserConstructionScript`)