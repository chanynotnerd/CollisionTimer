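; Actor Blueprint that moves its Cube component in a looping square path on the local XZ plane.
; On Tick, while Isplay is true, a MoveType state switch nudges the cube a fixed step right, up, left or down, advancing to the next direction when its relative location passes a bound.
; Movement is per frame without delta time.
; DoPlay and DoStop call their parent versions and toggle Isplay.
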(event `self.ReceiveTick`
  (params (DeltaSeconds :type "Float (single-precision)"))
  (bind (_relativelocation_x _relativelocation_y _relativelocation_z) (`KismetMathLibrary.BreakVector` (`SceneComponent.RelativeLocation` (`self.Cube`))))
  (bind _relativelocation_x_2 (`KismetMathLibrary.BreakVector` (`SceneComponent.RelativeLocation` (`self.Cube`))))
  (bind (_relativelocation_x_3 _relativelocation_y_2 _relativelocation_z_2) (`KismetMathLibrary.BreakVector` (`SceneComponent.RelativeLocation` (`self.Cube`))))
  (bind _relativelocation_x_4 (`KismetMathLibrary.BreakVector` (`SceneComponent.RelativeLocation` (`self.Cube`))))
  (if (`self.Isplay`)
    (switch `/Game/StartUnreal/EN_MoveType` (`self.MoveType`)
      (:`NewEnumerator0`
        ;[1 1 1] 오른쪽 이동
        (`SceneComponent.K2_AddRelativeLocation` (`self.Cube`) (1.0 0.0 0.0) false false)
        (if (> _relativelocation_x_2 100.0)
          (set `self.MoveType` "NewEnumerator1")))
      (:`NewEnumerator1`
        ;[1 1 1] 위로 이동
        (`SceneComponent.K2_AddRelativeLocation` (`self.Cube`) (0.0 0.0 1.0) false false)
        (if (> _relativelocation_z_2 100.0)
          (set `self.MoveType` "NewEnumerator2")))
      (:`NewEnumerator2`
        ;[1 1 1] 왼쪽 이동
        (`SceneComponent.K2_AddRelativeLocation` (`self.Cube`) (-1.0 0.0 0.0) false false)
        (if (< _relativelocation_x_4 0.0)
          (set `self.MoveType` "NewEnumerator3")))
      (:`NewEnumerator3`
        ;[1 1 1] 아래로 이동
        (`SceneComponent.K2_AddRelativeLocation` (`self.Cube`) (0.0 0.0 -1.0) false false)
        (if (< _relativelocation_z 0.0)
          (set `self.MoveType` "NewEnumerator0"))))))

(fn `DoPlay`
  (`parent.DoPlay`)
  (set `self.Isplay` true))

(fn `DoStop`
  (`parent.DoStop`)
  (set `self.Isplay` false))

(fn `UserConstructionScript`)